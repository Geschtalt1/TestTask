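; BP_RopeSphere_2 is a test-task actor with a sphere and a cable that can be raised or lowered.
; BeginPlay nudges the sphere sideways once.
; Up and Down events share identical logic, offsetting the Cable component vertically by input value times Speed, while ChangeSpeed updates Speed through a clamping setter.
; The cable-length function is an empty stub, and the PhysicsConstraint offset is unconnected.
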(event Custom|Up
  (params (Value :type Float%20%28double-precision%29))
  ;[0 0 0] Поднять веревку
  (Transformation|AddLocalOffset (Variables|Default|GetCable) (Math|Vector|MakeVector 0.0 0.0 (* Value (Variables|Setting|GetSpeed))) false false))

(event Custom|Down
  (params (Value :type Float%20%28double-precision%29))
  ;[0 0 0] Отпустить веревку
  (Transformation|AddLocalOffset (Variables|Default|GetCable) (Math|Vector|MakeVector 0.0 0.0 (* Value (Variables|Setting|GetSpeed))) false false))

(event Custom|Change%20Speed
  (params (NewParam :type Float%20%28double-precision%29))
  ;[0 0 0] Изменить скорость
  (CallFunction|SetSpeed NewParam))

(event EventBeginPlay
  (Transformation|AddLocalOffset (Variables|Default|GetSphere) "25.000000,52.000000, 0" false false)
  (Utilities|FlowControl|Delay 3.0))

(event EventTick
  (params (DeltaSeconds :type Float%20%28single-precision%29)))

(fn ConstructionScript)

(fn SetSpeed
  (params (NewSpeed :type Float%20%28double-precision%29))
  (Variables|Setting|SetSpeed (Math|Float|Clamp(Float) NewSpeed 1.0 2.0))
  (return))

(fn SetLenghtCable
  (params (NewLenght :type Float%20%28double-precision%29)))