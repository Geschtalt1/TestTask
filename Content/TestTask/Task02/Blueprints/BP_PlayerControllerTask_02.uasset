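; Player controller for test Task 02, meant to raise and lower rope-hung spheres through RopeUp and RopeDown axis input.
; Its construction script caches all BP_RopeSphere actors in AllSphere, and GetSphere holds an unused lookup by ID.
; Both axis events are empty: the Up and Down calls on sphere 0 are disconnected, as are two unfinished speed-change branches.
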(event Input|AxisEvents|InputAxisRopeUp
  (params (AxisValue :type Float%20%28single-precision%29))
  ;[0 0 0] Задание 2
  ;;[0.5 0.5 0.5] Веревка затягивается, шар поднимается вверх
)

(event Input|AxisEvents|InputAxisRopeDown
  (params (AxisValue :type Float%20%28single-precision%29))
  ;[0 0 0] Задание 2
  ;;[0.5 0.5 0.5] Веревка удлиняется, шар опускается вниз
)

(fn ConstructionScript
  (CallFunction|Initialization))

(fn Initialization
  (bind _outactors (Actor|GetAllActorsOfClass "/Game/TestTask/Task02/Blueprints/BP_RopeSphere.BP_RopeSphere_C"))
  (Variables|Default|SetAll%20Sphere _outactors))