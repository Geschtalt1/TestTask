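; BP_RopeSphere is a rope-and-sphere actor whose component B can be raised and lowered vertically.
; BeginPlay offsets the sphere and records B's start location plus an upper endpoint 390 units above it.
; Up and Down events offset B by input value times Speed unless it is within tolerance of the matching endpoint.
; Speed changes are clamped and printed on screen each tick; the cable-length function is an empty stub.
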(event Custom|Up
  (params (Value :type Float%20%28double-precision%29))
  ;[0 0 0] Поднять веревку
  (if (not (Utilities|Operators|EqualEqual (Transformation|GetWorldLocation (Variables|Default|GetB)) (Variables|Private|GetEndLocation) 1.0))
    (Transformation|AddLocalOffset (Variables|Default|GetB) (Math|Vector|MakeVector 0.0 0.0 (* Value (Variables|Setting|GetSpeed))) false false)))

(event Custom|Down
  (params (Value :type Float%20%28double-precision%29))
  ;[0 0 0] Отпустить веревку
  (if (not (Utilities|Operators|EqualEqual (Transformation|GetWorldLocation (Variables|Default|GetB)) (Variables|Private|GetBeginLocation) 1.0))
    (Transformation|AddLocalOffset (Variables|Default|GetB) (Math|Vector|MakeVector 0.0 0.0 (* Value (Variables|Setting|GetSpeed))) false false)))

(event Custom|Change%20Speed
  (params (NewParam :type Float%20%28double-precision%29))
  ;[0 0 0] Изменить скорость
  (CallFunction|SetSpeed NewParam))

(event EventBeginPlay
  ;[0 0 0] Иницилизация
  (Transformation|AddLocalOffset (Variables|Default|GetSphere) "25.000000,52.000000, 0" false false)
  (bind _output_get (Variables|Private|SetBeginLocation (Transformation|GetWorldLocation (Variables|Default|GetB))))
  (Variables|Private|SetEndLocation (+ _output_get "0,0,390.000000")))

(event EventTick
  (params (DeltaSeconds :type Float%20%28single-precision%29))
  (Development|PrintString (Utilities|String|Append "Current Select Speed:" (Utilities|String|ToString(Float) (Variables|Setting|GetSpeed))) true true "(R=0.000000,G=1.000000,B=0.151564,A=1.000000)" 0.0))

(fn ConstructionScript)

(fn SetSpeed
  (params (NewSpeed :type Float%20%28double-precision%29))
  (Variables|Setting|SetSpeed (Math|Float|Clamp(Float) NewSpeed 1.0 2.0))
  (return))

(fn SetLenghtCable
  (params (NewLenght :type Float%20%28double-precision%29)))