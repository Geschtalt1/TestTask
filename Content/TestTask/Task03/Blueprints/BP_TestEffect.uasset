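; BP_TestEffect fades a set of lights (AllLight) in and out at a caller-supplied Speed.
; BeginPlay caches each light's intensity as its maximum after a zero-length delay.
; ShowLights and HideLights cancel the opposite looping timer and start one at the current frame delta, stepping intensity toward that maximum or zero.
; Never-reset counters of finished-light hits stop each timer upon equalling the last array index.
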(event Custom|ShowLights
  (params (Speed :type Float%20%28double-precision%29))
  ;[0 0 0] Показать свет
  (Variables|Private|SetSpeed Speed)
  (Utilities|Time|ClearandInvalidateTimerbyHandle (Variables|Timer|GetTimerOff))
  (bind _returnvalue (Utilities|Time|SetTimerbyFunctionName 0 "LightOn" (Utilities|Time|GetWorldDeltaSeconds) true))
  (Variables|Timer|SetTimerOn _returnvalue))

(event Custom|HideLights
  (params (Speed :type Float%20%28double-precision%29))
  ;[0 0 0] Погасить свет
  (Variables|Private|SetSpeed Speed)
  (Utilities|Time|ClearandInvalidateTimerbyHandle (Variables|Timer|GetTimerOn))
  (bind _returnvalue (Utilities|Time|SetTimerbyFunctionName 0 "LightOff" (Utilities|Time|GetWorldDeltaSeconds) true))
  (Variables|Timer|SetTimerOff _returnvalue))

(event EventBeginPlay
  ;[0 0 0] Добавляем в массив, яркость по дефолту
  (Utilities|FlowControl|Delay 0.0)
  (for _array_element (Variables|Array|GetAll%20Light)
    (Utilities|IsValid _array_element
      (:Is%20Valid
        (Utilities|Array|Add (Variables|Array|GetIntensive%20Base) (Variables|/Script/Engine.LightComponentBase|GetIntensity _array_element))))))

(event EventTick
  (params (DeltaSeconds :type Float%20%28single-precision%29)))

(fn ConstructionScript)

(fn Lighton
  (for (_array_element _array_index) (Variables|Array|GetAll%20Light)
    (LocalVariables|SetID _array_index)
    (LocalVariables|SetLamp _array_element)
    ;[0 0 0] Если яркость лампочки не >= Intensive Base, то увеличиваем яркость
    (Utilities|IsValid (LocalVariables|GetLamp)
      (:Is%20Valid
        (if (not (>= (Variables|/Script/Engine.LightComponentBase|GetIntensity (LocalVariables|GetLamp)) (Utilities|Array|Get(acopy) (Variables|Array|GetIntensive%20Base) (LocalVariables|GetID))))
          ;[0 0 0] Вычитаем с помощью скорости, увелечение, новое значение яркости
          (Rendering|Components|Light|SetIntensity (LocalVariables|GetLamp) (Math|Float|Clamp(Float) (+ (Variables|/Script/Engine.LightComponentBase|GetIntensity (LocalVariables|GetLamp)) (Variables|Private|GetSpeed)) 0.0 (Utilities|Array|Get(acopy) (Variables|Array|GetIntensive%20Base) (LocalVariables|GetID))))
          (else
            ;[0 0 0] Когда яркость лампочки достигла дефолтного значения, прибовляем единицу в Count Light On и сравниваем с последним индексом в массиве для того что бы понять  все ли лампочки загорелись, если все отключаем таймер
            (bind _result (Math|Integer|IncrementInt (LocalVariables|GetCount%20Light%20On))
              (:%20%20
                (if (== _result (Utilities|Array|LastIndex (Variables|Array|GetAll%20Light)))
                  (Utilities|Time|ClearandInvalidateTimerbyHandle (Variables|Timer|GetTimerOn))
                  (Development|PrintString "Light On Successful!" true true "(R=0.000000,G=1.000000,B=0.000000,A=1.000000)"))))))))))

(fn LightOff
  ;[0 0 0] Инициализация
  (for (_array_element _array_index) (Variables|Array|GetAll%20Light)
    (LocalVariables|SetID _array_index)
    (LocalVariables|SetLamp _array_element)
    (Utilities|IsValid (LocalVariables|GetLamp)
      (:Is%20Valid
        ;[0 0 0] Если яркость лампочки не <= 0, то уменьшаем яркость
        (if (not (<= (Variables|/Script/Engine.LightComponentBase|GetIntensity (LocalVariables|GetLamp)) 0.0))
          ;[0 0 0] Вычитаем с помощью скорости, уменьшения, новое значение яркости
          (Rendering|Components|Light|SetIntensity (LocalVariables|GetLamp) (Math|Float|Clamp(Float) (- (Variables|/Script/Engine.LightComponentBase|GetIntensity (LocalVariables|GetLamp)) (Variables|Private|GetSpeed)) 0.0 (Utilities|Array|Get(acopy) (Variables|Array|GetIntensive%20Base) (LocalVariables|GetID))))
          (else
            ;[0 0 0] Когда яркость лампочки достигла 0, прибовляем единицу в Count Light Off и сравниваем с последним индексом в массиве для того что бы понять  все ли лампочки потухли, если все отключаем таймер
            (bind _result (Math|Integer|IncrementInt (LocalVariables|GetCount%20Light%20off%20))
              (:%20%20
                (if (== _result (Utilities|Array|LastIndex (Variables|Array|GetAll%20Light)))
                  (Utilities|Time|ClearandInvalidateTimerbyHandle (Variables|Timer|GetTimerOff))
                  (Development|PrintString "Light Off Successful!" true true "(R=0.000000,G=1.000000,B=0.000000,A=1.000000)"))))))))))