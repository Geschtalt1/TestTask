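; Events manager that shows or hides lights on cube and sphere effect actors at a given speed.
; The construction script caches all BP_Cube and BP_Sphere_01 actors.
; ExecuteEvent picks the type, requests index 0 through a getter, then calls ShowLights or HideLights, printing errors for unmatched selections.
; A timed demo sequence exists in the event graph but is disconnected from the empty BeginPlay.
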(event EventBeginPlay
  ;[0 0 0] Пример
)

(fn ConstructionScript
  (bind _outactors (Actor|GetAllActorsOfClass "/Game/TestTask/Task03/Blueprints/Actor/BP_Cube.BP_Cube_C"))
  (Variables|TArray|SetCube _outactors)
  (bind _outactors_2 (Actor|GetAllActorsOfClass "/Game/TestTask/Task03/Blueprints/Actor/BP_Sphere_01.BP_Sphere_01_C"))
  (Variables|TArray|SetSphere _outactors_2))

(fn ExecuteEvent
  (params (EffectName :type String) (Event :type String) (Speed :type Float%20%28double-precision%29))
  ;[0 0 0] Выбираем у какого типа объекта будим настраивать свет
  (switch string EffectName
    (:Default
      ;[0 0 0] Если объект не выбран
      (Development|PrintString "Object NULL!!!" true true "(R=1.000000,G=0.000000,B=0.000000,A=1.000000)"))
    (:Sphere
      (bind _output_get (LocalVariables|SetEffectLocal (Utilities|GetSphere)))
      (Utilities|IsValid _output_get
        (:Is%20Valid
          ;[0 0 0] Выбираем Показать или Скрыть свет
          (switch string Event :!label _label
            (:Default
              ;[0 0 0] Если евент не выбран
              (Development|PrintString "Event NULL!!!" true true "(R=1.000000,G=0.000000,B=0.000000,A=1.000000)"))
            (:ShowLights
              (Default|ShowLights (LocalVariables|GetEffectLocal) Speed))
            (:HideLight
              (Default|HideLights (LocalVariables|GetEffectLocal) Speed))))))
    (:Cube
      (bind _output_get_2 (LocalVariables|SetEffectLocal (Utilities|GetCube)))
      (Utilities|IsValid _output_get_2
        (:Is%20Valid
          (goto _label))))))