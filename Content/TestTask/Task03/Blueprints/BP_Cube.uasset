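; BP_Cube is an actor Blueprint with three light components, SL01 to SL03, set up at construction.
; Its construction script collects the lights into the AllLight array and sets each one's intensity to the shared IntensityBase value.
; The parent construction script runs afterward, once the lights are registered and configured.
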(fn ConstructionScript
  (Utilities|Array|Add (Variables|Default|GetAll%20Light) (Variables|Default|GetSL_01))
  (Utilities|Array|Add (Variables|Default|GetAll%20Light) (Variables|Default|GetSL_02))
  (Utilities|Array|Add (Variables|Default|GetAll%20Light) (Variables|Default|GetSL_03))
  (Rendering|Components|Light|SetIntensity (Variables|Default|GetSL_01) (Variables|Default|GetIntensity%20Base))
  (|CallParentFunction))