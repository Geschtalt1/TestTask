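; BP_Sphere_01 is an actor whose point light and spot light can be faded in and out.
; The construction script starts both lights at IntensityBase.
; ShowLights and HideLights store a Speed and start looping timers at frame-delta intervals.
; These call LightOn or LightOff, stepping intensity by Speed until both lights reach IntensityBase or zero, then clearing their own timer; neither event cancels the opposite fade.
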(event EventShowLights
  (params (Speed :type Float%20%28double-precision%29))
  ;[0 0 0] Показать свет
  (Variables|Default|SetSpeed Speed)
  (bind _returnvalue (Utilities|Time|SetTimerbyFunctionName 0 "LightOn" (Utilities|Time|GetWorldDeltaSeconds) true))
  (Variables|Default|SetTimerOn _returnvalue))

(event EventHideLights
  (params (Speed :type Float%20%28double-precision%29))
  ;[0 0 0] Погасить свет
  (Variables|Default|SetSpeed Speed)
  (bind _returnvalue (Utilities|Time|SetTimerbyFunctionName 0 "LightOff" (Utilities|Time|GetWorldDeltaSeconds) true))
  (Variables|Default|SetTimerOff _returnvalue))

(fn ConstructionScript
  (Rendering|Components|Light|SetIntensity (Variables|Default|GetSL_01) (Variables|Default|GetIntensity%20Base))
  (Rendering|Components|Light|SetIntensity (Variables|Default|GetPL_01) (Variables|Default|GetIntensity%20Base))
  (|CallParentFunction))

(fn LightOff
  (bind _sl_01 (Variables|Default|GetSL_01))
  (bind _pl_01 (Variables|Default|GetPL_01))
  (if (not (and (<= (Variables|/Script/Engine.LightComponentBase|GetIntensity (Variables|Default|GetPL_01)) 0.0) (<= (Variables|/Script/Engine.LightComponentBase|GetIntensity (Variables|Default|GetSL_01)) 0.0)))
    (Rendering|Components|Light|SetIntensity _pl_01 (- (Variables|/Script/Engine.LightComponentBase|GetIntensity _pl_01) (Variables|Default|GetSpeed)))
    (Rendering|Components|Light|SetIntensity _sl_01 (- (Variables|/Script/Engine.LightComponentBase|GetIntensity _sl_01) (Variables|Default|GetSpeed)))
    (else
      (Utilities|Time|ClearandInvalidateTimerbyHandle (Variables|Default|GetTimerOff)))))

(fn Lighton
  (bind _sl_01 (Variables|Default|GetSL_01))
  (bind _intensity_base (Variables|Default|GetIntensity%20Base))
  (bind _pl_01 (Variables|Default|GetPL_01))
  (if (not (and (>= (Variables|/Script/Engine.LightComponentBase|GetIntensity (Variables|Default|GetPL_01)) _intensity_base) (>= (Variables|/Script/Engine.LightComponentBase|GetIntensity (Variables|Default|GetSL_01)) _intensity_base)))
    ;[0 0 0] Увиличиваем свет лапочке
    (Rendering|Components|Light|SetIntensity _pl_01 (+ (Variables|/Script/Engine.LightComponentBase|GetIntensity _pl_01) (Variables|Default|GetSpeed)))
    ;[0 0 0] Увеличиваем свет Spot light
    (Rendering|Components|Light|SetIntensity _sl_01 (+ (Variables|/Script/Engine.LightComponentBase|GetIntensity _sl_01) (Variables|Default|GetSpeed)))
    (else
      (Utilities|Time|ClearandInvalidateTimerbyHandle (Variables|Default|GetTimerOn)))))