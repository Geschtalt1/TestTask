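; Player controller for test Task 3 that lets the player pick a cube or sphere and show or hide its light through an events manager.
; Input actions set the target name, flip-flop the show/hide event name, and send both with a fixed speed to BP_EventsManager's ExecuteEvent.
; The Construction Script finds that manager with GetActorOfClass.
; Tick prints both current selections on screen as debug output.
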(event EventTick
  (params (DeltaSeconds :type Float%20%28single-precision%29))
  ;[0 0 0] Debug
  (Development|PrintString (Utilities|String|Append "Select Object:" (Variables|Default|GetSelect%20Object)) true true "(R=1.000000,G=0.000000,B=1.000000,A=1.000000)" 0.0)
  (Development|PrintString (Utilities|String|Append "Select Event:" (Variables|Default|GetSelect%20Event)) true true "(R=0.526000,G=0.000000,B=1.000000,A=1.000000)" 0.0))

(event Input|ActionEvents|InputActionShow/HiddenLight
  (params (Key :type Key%20Structure :default "None"))
  ;[0 0 0] Задание 3
  ;;[0 1 1] Выбрать евент
  (:Pressed
    (Utilities|FlowControl|FlipFlop
      (:A
        (Variables|Default|SetSelect%20Event "ShowLights"))
      (:B
        (Variables|Default|SetSelect%20Event "HideLight")))))

(event Input|ActionEvents|InputActionSelectCube
  (params (Key :type Key%20Structure :default "None"))
  ;[0 0 0] Задание 3
  ;;[0 1 1] Выбрать куб
  (:Pressed
    (Variables|Default|SetSelect%20Object "Cube")))

(event Input|ActionEvents|InputActionSelectSphere
  (params (Key :type Key%20Structure :default "None"))
  ;[0 0 0] Задание 3
  ;;[0 1 1] Выбрать сферу
  (:Pressed
    (Variables|Default|SetSelect%20Object "Sphere")))

(event Input|ActionEvents|InputActionLightOn/Off
  (params (Key :type Key%20Structure :default "None"))
  ;[0 0 0] Задание 3
  ;;[0 1 1] Включаем или отлючаем свет выбраному объекту
  (:Pressed
    (Utilities|IsValid (Variables|Default|GetEventsRef)
      (:Is%20Valid
        (Default|ExecuteEvent (Variables|Default|GetEventsRef) (Variables|Default|GetSelect%20Object) (Variables|Default|GetSelect%20Event) 5e+01)))))

(fn ConstructionScript
  (bind _returnvalue (Actor|GetActorOfClass "/Game/TestTask/Task03/Blueprints/BP_EventsManager.BP_EventsManager_C"))
  (Variables|Default|SetEventsRef _returnvalue))