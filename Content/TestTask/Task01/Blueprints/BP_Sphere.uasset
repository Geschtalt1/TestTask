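; BP_Sphere is a test-task actor whose sphere fades and glows while moving vertically between its placed position and a Height offset.
; BeginPlay records both positions and starts it opaque at the raised one.
; OpacityOn/Off move and fade it, while ShowGlow/HiddenGlow ramp emissive, each re-arming a frame-delta timer and cancelling its opposite.
; Helpers write the Opacity and Glow material parameters, and Tick always draws debug values and spheres.
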(event Custom|OpacityOn
  ;[0 0 0] Включить прозрачность
  (Variables|OpacitySphere|SetbIsOpacityOn? true)
  (if (Variables|OpacitySphere|GetbIsOpacityOff?) ; Отключаем анимацию ухода если она была включена
    (CallFunction|TimerDisable (Variables|Timer|GetTimerOpacityOff))
    (Variables|OpacitySphere|SetbIsOpacityOff? false))
  (if (not (>= (Variables|OpacitySphere|GetOpacity) 1.0))
    (CallFunction|OpacityChange (Utilities|AddOpacity)))
  (if (not (Utilities|Operators|EqualEqual (Transformation|GetActorLocation) (Variables|Default|GetEnd%20Position) 1.0))
    (Transformation|AddActorLocalOffset (Math|Vector|MakeVector 0.0 0.0 (* (Utilities|Time|GetWorldDeltaSeconds) 3e+01)) false false)
    (bind _returnvalue (Utilities|Time|SetTimerbyEvent (delegate Custom|OpacityOn) (Utilities|Time|GetWorldDeltaSeconds)))
    (Variables|Timer|SetTimerOpacityOn _returnvalue)
    (else
      (Variables|OpacitySphere|SetbIsOpacityOn? false)
      (CallFunction|TimerDisable (Variables|Timer|GetTimerOpacityOn)))))

(event Custom|OpacityOff
  ;[0 0 0] Выключить прозрачность
  (Variables|OpacitySphere|SetbIsOpacityOff? true)
  (if (Variables|OpacitySphere|GetbIsOpacityOn?) ; Отключаем анимацию появления если она была включена
    (CallFunction|TimerDisable (Variables|Timer|GetTimerOpacityOn))
    (Variables|OpacitySphere|SetbIsOpacityOn? false))
  (if (not (<= (Variables|OpacitySphere|GetOpacity) 0.0))
    (CallFunction|OpacityChange (Utilities|MinusOpacity)))
  (if (not (Utilities|Operators|EqualEqual (Transformation|GetActorLocation) (Variables|Default|GetOriginal%20Position) 1.0))
    (Transformation|AddActorLocalOffset (Math|Vector|MakeVector 0.0 0.0 (* (* (Utilities|Time|GetWorldDeltaSeconds) 3e+01) -1.0)) false false)
    (bind _returnvalue (Utilities|Time|SetTimerbyEvent (delegate Custom|OpacityOff) (Utilities|Time|GetWorldDeltaSeconds)))
    (Variables|Timer|SetTimerOpacityOff _returnvalue)
    (else
      (Variables|OpacitySphere|SetbIsOpacityOff? false)
      (CallFunction|TimerDisable (Variables|Timer|GetTimerOpacityOff)))))

(event Custom|Show%20Glow
  ;[0 0 0] Включить свечение
  (Variables|EmissiveSphere|SetbIsGlowOn? true)
  (if (Variables|EmissiveSphere|GetbIsGlowOff)
    (CallFunction|TimerDisable (Variables|Timer|GetTimerHiddenGlow))
    (Variables|EmissiveSphere|SetbIsGlowOff false))
  (if (not (>= (Variables|EmissiveSphere|GetEmissive) (Variables|Setting|GetMax%20Emissive)))
    (CallFunction|EmissiveChange (Utilities|AddEmissive))
    (bind _returnvalue (Utilities|Time|SetTimerbyEvent (delegate Custom|Show%20Glow) (Utilities|Time|GetWorldDeltaSeconds)))
    (Variables|Timer|SetTimerShowGlow _returnvalue)
    (else
      (Variables|EmissiveSphere|SetbIsGlowOn? false)
      (CallFunction|TimerDisable (Variables|Timer|GetTimerShowGlow)))))

(event Custom|Hidden%20Glow
  ;[0 0 0] Выключить свечение
  (Variables|EmissiveSphere|SetbIsGlowOff true)
  (if (Variables|EmissiveSphere|GetbIsGlowOn?)
    (CallFunction|TimerDisable (Variables|Timer|GetTimerShowGlow))
    (Variables|EmissiveSphere|SetbIsGlowOn? false))
  (if (not (<= (Variables|EmissiveSphere|GetEmissive) 0.0))
    (CallFunction|EmissiveChange (Utilities|MinusEmissive))
    (bind _returnvalue (Utilities|Time|SetTimerbyEvent (delegate Custom|Hidden%20Glow) (Utilities|Time|GetWorldDeltaSeconds)))
    (Variables|Timer|SetTimerHiddenGlow _returnvalue)
    (else
      (Variables|EmissiveSphere|SetbIsGlowOff false)
      (CallFunction|TimerDisable (Variables|Timer|GetTimerHiddenGlow)))))

(event EventBeginPlay
  ;[0 0 0] Инициализация
  (CallFunction|Initialization))

(event EventTick
  (params (DeltaSeconds :type Float%20%28single-precision%29))
  ;[0 0 0] Debug
  (CallFunction|Debug true))

(fn ConstructionScript)

(fn OpacityChange
  (params (Opacity%20Value :type Float%20%28single-precision%29))
  (Rendering|Material|SetScalarParameterValueonMaterials (Variables|Default|GetSphere) "Opacity" (Math|Float|Clamp(Float) Opacity%20Value))
  (bind _output_get (Variables|OpacitySphere|SetOpacity Opacity%20Value))
  (return _output_get))

(fn EmissiveChange
  (params (Glow%20Valuee :type Float%20%28single-precision%29))
  (Rendering|Material|SetScalarParameterValueonMaterials (Variables|Default|GetSphere) "Glow" (Math|Float|Clamp(Float) Glow%20Valuee 0.0 (Variables|Setting|GetMax%20Emissive)))
  (bind _output_get (Variables|EmissiveSphere|SetEmissive Glow%20Valuee))
  (return _output_get))

(fn Initialization
  ;[0 0 0] При старте выставляем по умолчанию opacity 1.0, emissive 10.0 и записываем начальную позицию и позицию куда нужно двигаться
  (CallFunction|OpacityChange 1.0)
  (CallFunction|EmissiveChange (Variables|EmissiveSphere|GetEmissive))
  (Variables|Default|SetOriginal%20Position (Transformation|GetWorldLocation (Variables|Default|GetSphere)))
  (bind _output_get (Variables|Default|SetEnd%20Position (+ (Variables|Default|GetOriginal%20Position) (Math|Vector|MakeVector 0.0 0.0 (Variables|Setting|GetHeight)))))
  (Transformation|SetActorLocation _output_get false false))

(fn TimerDisable
  (params (Timer%20Handle :type Timer%20Handle%20Structure))
  (Utilities|Time|PauseTimerbyHandle Timer%20Handle)
  (Utilities|Time|ClearandInvalidateTimerbyHandle Timer%20Handle))

(fn HeightSphereChange
  (params (Height :type Float%20%28double-precision%29))
  (Transformation|SetActorLocation (Math|Vector|MakeVector 0.0 0.0 Height) false false))

(fn Debug
  (params (bDebug? :type Boolean))
  (if bDebug?
    (Development|PrintString (Utilities|String|Append "Opacity:" (Utilities|String|ToString(Float) (Variables|OpacitySphere|GetOpacity))) true true "(R=0.000000,G=1.000000,B=0.000000,A=1.000000)" 0.0)
    (Development|PrintString (Utilities|String|Append "Emissive:" (Utilities|String|ToString(Float) (Variables|EmissiveSphere|GetEmissive))) true true "(R=0.000000,G=1.000000,B=0.000000,A=1.000000)" 0.0)
    (Rendering|Debug|DrawDebugSphere (Variables|Default|GetOriginal%20Position) 45.0 12 "(R=0.000000,G=1.000000,B=1.000000,A=1.000000)" 0.0)
    (Rendering|Debug|DrawDebugSphere (Transformation|GetActorLocation) 45.0 12 "(R=1.000000,G=1.000000,B=1.000000,A=1.000000)" 0.0)
    (Rendering|Debug|DrawDebugSphere (Variables|Default|GetEnd%20Position) 45.0 12 "(R=1.000000,G=0.000000,B=0.000000,A=1.000000)" 0.0)))