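; Test-task player controller that triggers fade and glow animations on a BP_Sphere actor through input actions.
; Its construction script caches every BP_Sphere in the level into AllSphere.
; Four input presses fetch index 0 through GetSphere, check validity, then call OpacityOn, OpacityOff, ShowGlow or HiddenGlow.
; The Get Sphere graph contains only an AllSphere lookup by ID, marked as unused.
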(event Input|ActionEvents|InputActionOpacityAnimationOn
  (params (Key :type Key%20Structure :default "None"))
  (bind _sphere (Utilities|GetSphere))
  ;[0 0 0] Задание 1
  ;;[0.5 0.5 0.5] Анимация появления
  (:Pressed
    (Utilities|IsValid _sphere
      (:Is%20Valid
        (Default|Opacityon _sphere)))))

(event Input|ActionEvents|InputActionOpacityAnimationOff
  (params (Key :type Key%20Structure :default "None"))
  (bind _sphere (Utilities|GetSphere))
  ;[0 0 0] Задание 1
  ;;[0.5 0.5 0.5] Анимация ухода
  (:Pressed
    (Utilities|IsValid _sphere
      (:Is%20Valid
        (Default|OpacityOff _sphere)))))

(event Input|ActionEvents|InputActionShowAnimationGlow
  (params (Key :type Key%20Structure :default "None"))
  (bind _sphere (Utilities|GetSphere))
  ;[0 0 0] Задание 1
  ;;[0.5 0.5 0.5] Показ анимации свечения
  (:Pressed
    (Utilities|IsValid _sphere
      (:Is%20Valid
        (Default|ShowGlow _sphere)))))

(event Input|ActionEvents|InputActionHideAnimationGlow
  (params (Key :type Key%20Structure :default "None"))
  (bind _sphere (Utilities|GetSphere))
  ;[0 0 0] Задание 1
  ;;[0.5 0.5 0.5] Скрытие анимации свечения
  (:Pressed
    (Utilities|IsValid _sphere
      (:Is%20Valid
        (Default|HiddenGlow _sphere)))))

(fn ConstructionScript
  (CallFunction|Initialization))

(fn Initialization
  (bind _outactors (Actor|GetAllActorsOfClass "/Game/TestTask/Task01/Blueprints/BP_Sphere.BP_Sphere_C"))
  (Variables|Default|SetAll%20Sphere _outactors))